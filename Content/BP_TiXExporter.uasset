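; BP_TiXExporter is a utility actor that exports the current scene or a single static mesh actor to a configured path.
; Boolean toggles build string lists of scene content types and mesh vertex attributes.
; Export Scene passes both lists and a mesh scale to ExportCurrentScene.
; Export Static Mesh passes the attribute list and scale to ExportStaticMeshActor when the target is valid, with no runtime event logic.
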(event EventBeginPlay)

(event Collision|EventActorBeginOverlap
  (params (OtherActor :type Actor%20Object%20Reference)))

(event EventTick
  (params (DeltaSeconds :type Float%20%28single-precision%29)))

(fn ConstructionScript)

(fn ExportScene
  (bind _options (CallFunction|GetStaticMeshExportOption))
  (bind _components (CallFunction|GetSceneExportOption))
  (Class|TiXExporterBPLibrary|ExportCurrentScene self (Variables|Settings|GetPath%20to%20Export) _components _options (Variables|Settings|GetMeshScale)))

(fn ExportStaticMesh
  (if (Utilities|IsValid (Variables|StaticMesh|GetStatic%20Mesh%20Actor))
    (bind _options (CallFunction|GetStaticMeshExportOption))
    (Class|TiXExporterBPLibrary|ExportStaticMeshActor (Variables|StaticMesh|GetStatic%20Mesh%20Actor) (Variables|Settings|GetPath%20to%20Export) _options (Variables|Settings|GetMeshScale))
    (Development|PrintString "Export static mesh done")))

(fn GetSceneExportOption
  (bind _exportscenecomponents (LocalVariables|GetExportSceneComponents))
  (Utilities|FlowControl|Sequence
    (:then_0
      (if (Variables|ExportScene|GetExportStaticMesh)
        (Utilities|Array|Add _exportscenecomponents "STATIC_MESH")))
    (:then_1
      (if (Variables|ExportScene|GetExportSkeletalMesh)
        (Utilities|Array|Add _exportscenecomponents "SKELETAL_MESH")))
    (:then_2
      (if (Variables|ExportScene|GetExportFoliageAndGrass)
        (Utilities|Array|Add _exportscenecomponents "FOLIAGE_AND_GRASS")))
    (:then_3
      (if (Variables|ExportScene|GetExportLandscape)
        (Utilities|Array|Add _exportscenecomponents "LANDSCAPE")))
    (:then_4
      (return (LocalVariables|GetExportSceneComponents)))))

(fn GetStaticMeshExportOption
  (bind _exportcomponents (LocalVariables|GetExportComponents))
  (Utilities|FlowControl|Sequence
    (:then_0
      (if (Variables|StaticMesh|GetPosition)
        (Utilities|Array|Add _exportcomponents "POSITION")))
    (:then_1
      (if (Variables|StaticMesh|GetNormal)
        (Utilities|Array|Add _exportcomponents "NORMAL")))
    (:then_2
      (if (Variables|StaticMesh|GetColor)
        (Utilities|Array|Add _exportcomponents "COLOR")))
    (:then_3
      (if (Variables|StaticMesh|GetTexCoord0)
        (Utilities|Array|Add _exportcomponents "TEXCOORD0")))
    (:then_4
      (if (Variables|StaticMesh|GetTexCoord1)
        (Utilities|Array|Add _exportcomponents "TEXCOORD1")))
    (:then_5
      (if (Variables|StaticMesh|GetTangent)
        (Utilities|Array|Add _exportcomponents "TANGENT")))
    (:then_6
      (return (LocalVariables|GetExportComponents)))))